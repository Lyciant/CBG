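; Base first-person player pawn that handles walking, mouse-look style camera control and jumping.
; Move axes feed AddMovementInput along the actor's forward and right vectors.
; Pitch input rotates only the FPV camera, clamped short of vertical, while yaw input turns the whole actor.
; Jump applies an upward velocity-change impulse to the capsule when a short downward Visibility line trace finds ground.
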(event `InputAction|Jump`
  (params (Key :type "Key Structure"))
  (bind (_returnvalue_x _returnvalue_y _returnvalue_z) (`KismetMathLibrary.BreakVector` (`self.K2_GetActorLocation`)))
  ;[1 1 1] Jumping
  (:`Pressed`
    (bind (_outhit _returnvalue) (`KismetSystemLibrary.LineTraceSingle` (`self.K2_GetActorLocation`) (`KismetMathLibrary.MakeVector` _returnvalue_x _returnvalue_y (+ _returnvalue_z -70.0)) "TraceTypeQuery1"))
    (if _returnvalue
      (`PrimitiveComponent.AddImpulse` (`self.Capsule`) (`KismetMathLibrary.MakeVector` 0.0 0.0 (`self.Jump Force`)) "None" true))))

(event `InputAxis|MoveForwards`
  (params (AxisValue :type "Float (single-precision)"))
  ;[1 1 1] Pawn Movement
  (`self.AddMovementInput` (`self.GetActorForwardVector`) AxisValue))

(event `InputAxis|MoveRight`
  (params (AxisValue :type "Float (single-precision)"))
  ;[1 1 1] Pawn Movement
  (`self.AddMovementInput` (`self.GetActorRightVector`) AxisValue))

(event `InputAxis|CameraPitch`
  (params (AxisValue :type "Float (single-precision)"))
  (bind (_returnvalue_roll _returnvalue_pitch _returnvalue_yaw) (`KismetMathLibrary.BreakRotator` (`SceneComponent.GetSocketRotation` (`self.Camera_FPV`) "None")))
  ;[1 1 1] Camera Movement
  (`SceneComponent.K2_SetRelativeRotation` (`self.Camera_FPV`) (`KismetMathLibrary.MakeRotator` (`KismetMathLibrary.ClampAngle` _returnvalue_roll) (`KismetMathLibrary.ClampAngle` (+ _returnvalue_pitch AxisValue) -89.0 89.0)) false false))

(event `InputAxis|CameraYaw`
  (params (AxisValue :type "Float (single-precision)"))
  (bind (_returnvalue_roll _returnvalue_pitch _returnvalue_yaw) (`KismetMathLibrary.BreakRotator` (`SceneComponent.GetSocketRotation` (`self.Camera_FPV`) "None")))
  ;[1 1 1] Camera Movement
  (`self.K2_SetActorRotation` (`KismetMathLibrary.MakeRotator` 0.0 0.0 (+ _returnvalue_yaw AxisValue))))

(fn `UserConstructionScript`)